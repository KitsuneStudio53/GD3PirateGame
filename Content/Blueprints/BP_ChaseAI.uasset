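; Chase AI pawn that wanders randomly and pursues any pawn it spots through PawnSensing.
; Roaming starts on BeginPlay, moves to random reachable points around itself and repeats after each successful move.
; A sighting starts a move toward the seen pawn and resets a retriggerable delay, which returns it to roaming once sightings stop.
; ToggleMovement freezes it while flagged as seen and restores walking otherwise.
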(event OnSeePawn(PawnSensing)
  (params (Pawn :type Pawn%20Object%20Reference))
  ;[1 1 1] Chase Player when seen
  (Utilities|FlowControl|Sequence
    (:then_0
      (AI|AIMoveTo self "0, 0, 0" Pawn 5.0 false))
    (:then_1
      (Utilities|FlowControl|RetriggerableDelay 3.0)
      (CallFunction|AIRoam))))

(event Custom|AI_Roam
  ;[1 1 1] Roam around when not doing anything
  (AI|AIMoveTo self (.RandomLocation (AI|Navigation|GetRandomReachablePointinRadius (Transformation|GetActorLocation) 5e+03 0 0)) 0 5.0 false
    (:OnSuccess
      (Utilities|FlowControl|Delay 0.1)
      (CallFunction|AIRoam))))

(event EventBeginPlay
  (CallFunction|AIRoam))

(event EventToggleMovement
  (params (isSeen :type Boolean))
  (bind _charactermovement (Variables|Character|GetCharacterMovement))
  (if isSeen
    (Pawn|Components|CharacterMovement|DisableMovement _charactermovement)
    (else
      (Pawn|Components|CharacterMovement|SetMovementMode _charactermovement "MOVE_Walking" 0))))

(fn ConstructionScript)